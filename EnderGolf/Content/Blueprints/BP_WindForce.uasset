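; BP_WindForce is a wind actor that pushes EnderProjectile actors while they overlap it.
; Each Tick it applies a continuous force to a PrimitiveComponent on every overlapping projectile, along the Arrow component's forward vector scaled by ForceValue.
; The force is mass-dependent, as AccelChange is off.
; Characters are unaffected, since their cast and query nodes are disconnected leftovers, as are an older fixed-force branch and an impulse node.
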(event EventBeginPlay)

(event Collision|EventActorBeginOverlap
  (params (OtherActor :type Actor%20Object%20Reference)))

(event EventTick
  (params (DeltaSeconds :type Float%20%28single-precision%29))
  (for _array_element (Collision|GetOverlappingActors "/Script/EnderGolf.EnderProjectile" :!class /Script/Engine.Actor)
    (Physics|AddForce (Actor|GetComponentbyClass _array_element "/Script/Engine.PrimitiveComponent") (* (Math|Vector|GetForwardVector (Variables|Default|GetArrow)) (Variables|Default|GetForceValue)) "None" false)))

(fn ConstructionScript)